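; Test character for a task exercising a replication UObject and a runtime-spawned component in multiplayer.
; On BeginPlay the server constructs a BP_ObjectForReplication; T randomizes or toggles its values locally, and Tick prints them with the character's name.
; Y on the server replaces the dynamic static mesh component with a new camera mesh, and every Y press prints that component's name if valid.
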(event `self.ReceiveBeginPlay`
  (if (`KismetSystemLibrary.IsServer`)
    (`self.ConstructUobject`)))

(event `ConstructUobject`
  (bind _returnvalue (`|GenericCreateObject` "/Game/Task_04/BP_ObjectForReplication.BP_ObjectForReplication_C"))
  (set `self.UobjectRef` _returnvalue))

(event `Key|T`
  (params (Key :type "Key Structure"))
  (:`Pressed`
    (`self.ChangeVars`)))

(event `ChangeVars`
  (bind _uobjectref (`self.UobjectRef`)
    (:`then`
      (set `/Game/Task_04/BP_ObjectForReplication.Value1` (not (`/Game/Task_04/BP_ObjectForReplication.Value1` _uobjectref)) _uobjectref)
      (set `/Game/Task_04/BP_ObjectForReplication.Value2` (`KismetMathLibrary.RandomFloat`) _uobjectref)
      (set `/Game/Task_04/BP_ObjectForReplication.Value3` (`KismetMathLibrary.RandomInteger` 100) _uobjectref))
    (:`else`)))

(event `self.ReceiveTick`
  (params (DeltaSeconds :type "Float (single-precision)"))
  (`self.PrintVars`))

(event `PrintVars`
  (bind _uobjectref (`self.UobjectRef`)
    (:`then`
      (`KismetSystemLibrary.PrintText` (`|FormatText` "Value 1 = {1} \nValue 2 = {2} \nValue 3 = {3}" (`/Game/Task_04/BP_ObjectForReplication.Value1` _uobjectref) (`/Game/Task_04/BP_ObjectForReplication.Value2` _uobjectref) (`/Game/Task_04/BP_ObjectForReplication.Value3` _uobjectref)) true true (struct :`R` 1.0 :`B` 0.440944 :`A` 1.0) 0.0)
      (`KismetSystemLibrary.PrintString` (`KismetSystemLibrary.GetDisplayName` self) true true (struct :`G` 0.66 :`B` 1.0 :`A` 1.0) 0.0))
    (:`else`)))

(event `Key|Y`
  (params (Key :type "Key Structure"))
  (:`Pressed`
    (if (`KismetSystemLibrary.IsServer`)
      (`self.Spawn Component`))
    (`self.PrintComponentLink`)))

(event `Spawn Component`
  (bind _dynamiccomponent (`self.DynamicComponent`))
  (`|ExecutionSequence`
    (:`then_0`
      (`/Engine/EditorBlueprintResources/StandardMacros.IsValid` _dynamiccomponent
        (:`Is Valid`
          (`ActorComponent.K2_DestroyComponent` _dynamiccomponent)
          (set `self.DynamicComponent` null))))
    (:`then_1`
      (bind _returnvalue (`|AddComponentByClass` "/Script/Engine.StaticMeshComponent" false (`KismetMathLibrary.MakeTransform` (200.0 0.0 0.0) (struct :`Yaw` 180.0))))
      (bind _output_get (set `self.DynamicComponent` _returnvalue))
      (`StaticMeshComponent.SetStaticMesh` _output_get "/Engine/EditorMeshes/MatineeCam_SM.MatineeCam_SM"))))

(event `PrintComponentLink`
  (bind _dynamiccomponent (`self.DynamicComponent`)
    (:`then`
      (`KismetSystemLibrary.PrintString` (`KismetSystemLibrary.GetDisplayName` _dynamiccomponent)))
    (:`else`)))

(fn `UserConstructionScript`)