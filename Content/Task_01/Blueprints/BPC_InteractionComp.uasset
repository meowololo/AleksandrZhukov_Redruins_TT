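; Actor component for a Character that finds the interactable the player is looking at and tells it to highlight.
; At BeginPlay it adds an overlap sphere that tracks actors returned by an identify message.
; Each tick it scores them by dot product from a point ahead of the camera, picking the best above a threshold.
; A visibility trace from the owner must hit that actor before the highlight message is sent.
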(event `self.ReceiveBeginPlay`
  (`self.InteractionSetup`))

(event `self.ReceiveTick`
  (params (DeltaSeconds :type "Float (single-precision)"))
  (bind _nearestactor (`self.FindLookAtObject`))
  (bind _output_get (set `self.Nearest Actor` _nearestactor))
  (`/Engine/EditorBlueprintResources/StandardMacros.IsValid` _output_get
    (:`Is Valid`
      (bind _noobstacles (`self.TraceForObstacles`))
      (if _noobstacles
        (message `/Game/Task_01/Blueprints/BPI_Interaction.HighlightForInteract` (`self.Nearest Actor`))))))

(fn `AddDetectedInteractActor`
  (params (DetectedActor :type "Actor Object Reference"))
  (`/Engine/EditorBlueprintResources/StandardMacros.IsValid` DetectedActor
    (:`Is Valid`
      (if (== (`KismetArrayLibrary.Array_Find` (`self.InteractActorsInRange`) (`local.DetectedActor`)) -1)
        (`KismetArrayLibrary.Array_Add` (`self.InteractActorsInRange`) (`local.DetectedActor`))))))

(fn `FindLookAtObject`
  (returns (NearestActor :type "Actor Object Reference"))
  (locals (BiggerLookingCoef :type "Float (double-precision)") (ActorToInteractWith :type "Actor Object Reference"))
  (bind _charactercamera (`self.CharacterCamera`))
  (`BlueprintMapLibrary.Map_Clear` (`self.LookAtCoefs`))
  (set `local.BiggerLookingCoef` 0.0)
  (for _array_element (`self.InteractActorsInRange`)
    (`BlueprintMapLibrary.Map_Add` (`self.LookAtCoefs`) _array_element (`KismetMathLibrary.Dot_VectorVector` (`SceneComponent.GetForwardVector` (`self.CharacterCamera`)) (`KismetMathLibrary.GetForwardVector` (`KismetMathLibrary.FindLookAtRotation` (+ (`SceneComponent.K2_GetComponentLocation` _charactercamera) (* (`SceneComponent.GetForwardVector` _charactercamera) 200.0)) (`Actor.K2_GetActorLocation` _array_element))))))
  (bind _keys (`BlueprintMapLibrary.Map_Keys` (`self.LookAtCoefs`)))
  (for _array_element_2 _keys
    (bind _value (`BlueprintMapLibrary.Map_Find` (`self.LookAtCoefs`) _array_element_2))
    (if (> _value (`local.BiggerLookingCoef`))
      (set `local.BiggerLookingCoef` _value)
      (if (> (`local.BiggerLookingCoef`) 0.9)
        (set `local.ActorToInteractWith` _array_element_2)
        (else
          (set `local.ActorToInteractWith` null)))))
  (return (`local.ActorToInteractWith`)))

(fn `IdentifyActor`
  (returns (DetectedActor :type "Actor Object Reference"))
  (return null))

(fn `InteractionSetup`
  (bind _spherecollision (`self.SphereCollision`))
  (bind _showspherecollision (`self.ShowSphereCollision`))
  (bind _ascharacter (cast `Character` (`self.GetOwner`)))
  (bind _output_get (set `self.CharacterOwner` _ascharacter))
  (bind _returnvalue (`|AddComponentByClass` :`self` _output_get :`Class` "/Script/Engine.SphereComponent"))
  (set `self.SphereCollision` _returnvalue)
  (`SphereComponent.SetSphereRadius` _spherecollision (`self.CollisionSphereRadius`) true)
  (`SceneComponent.SetVisibility` _spherecollision _showspherecollision false)
  (`SceneComponent.SetHiddenInGame` _spherecollision (not _showspherecollision) false)
  (`PrimitiveComponent.SetCollisionResponseToAllChannels` _spherecollision "ECR_Overlap")
  (add `PrimitiveComponent.OnComponentBeginOverlap` _spherecollision (`|CreateDelegate` :!event `InteractSphereBeginOverlap`))
  (add `PrimitiveComponent.OnComponentEndOverlap` _spherecollision (`|CreateDelegate` :!event `InteractSphereEndOverlap`)))

(fn `InteractSphereBeginOverlap`
  (params (OverlappedComponent :type "PrimitiveComponent Object Reference") (OtherActor :type "Actor Object Reference") (OtherComp :type "PrimitiveComponent Object Reference") (OtherBodyIndex :type Integer) (bFromSweep :type Boolean) (SweepResult :type "HitResult Structure (by ref)"))
  (bind _detectedactor (message `/Game/Task_01/Blueprints/BPI_Interaction.IdentifyActor` OtherActor))
  (`self.AddDetectedInteractActor` _detectedactor)
  (return))

(fn `InteractSphereEndOverlap`
  (params (OverlappedComponent :type "PrimitiveComponent Object Reference") (OtherActor :type "Actor Object Reference") (OtherComp :type "PrimitiveComponent Object Reference") (OtherBodyIndex :type Integer))
  (bind _detectedactor (message `/Game/Task_01/Blueprints/BPI_Interaction.IdentifyActor` OtherActor))
  (`self.RemoveInteractActor` _detectedactor))

(fn `RemoveInteractActor`
  (params (ActorToRemove :type "Actor Object Reference"))
  (if (!= (`KismetArrayLibrary.Array_Find` (`self.InteractActorsInRange`) (`local.ActorToRemove`)) -1)
    (`KismetArrayLibrary.Array_RemoveItem` (`self.InteractActorsInRange`) (`local.ActorToRemove`))
    (return)))

(fn `TraceForObstacles`
  (returns (NoObstacles :type Boolean))
  (bind _outhit (`KismetSystemLibrary.LineTraceSingle` :`Start` (`Actor.K2_GetActorLocation` (`self.GetOwner`)) :`End` (`Actor.K2_GetActorLocation` (`self.Nearest Actor`)) :`TraceChannel` "TraceTypeQuery1" :`DrawTime` 0.1))
  (return (not (!= (`.HitActor` (`GameplayStatics.BreakHitResult` _outhit)) (`self.Nearest Actor`)))))