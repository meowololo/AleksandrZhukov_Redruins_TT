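; BP_Task_01_Actor is an interactable actor that shows a clue when highlighted and changes its sphere's material on interaction.
; HighlightforInteract shows WInteractionClue and uses a short retriggerable delay to hide it once highlight calls stop arriving.
; Interact applies BasicAsset01 to the sphere, and IdentifyActor returns the actor itself to callers.
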(event `/Game/Task_01/Blueprints/BPI_Interaction.HighlightForInteract`
  (`SceneComponent.SetVisibility` (`self.W_InteractionClue`) true false)
  (`KismetSystemLibrary.RetriggerableDelay` 0.1)
  (`SceneComponent.SetVisibility` (`self.W_InteractionClue`) false false))

(event `/Game/Task_01/Blueprints/BPI_Interaction.Interact`
  (`PrimitiveComponent.SetMaterial` (`self.Sphere`) 0 "/Engine/MapTemplates/Materials/BasicAsset01.BasicAsset01"))

(fn `IdentifyActor`
  (returns (DetectedActor :type "Actor Object Reference"))
  (return self))

(fn `UserConstructionScript`)