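; BP_Task_06_Actor is a homing projectile that steers toward the first BP_Task_06_Target found on BeginPlay.
; Each Tick it rebuilds ProjectileMovement velocity from a fixed forward speed plus a pull toward the target.
; A dot product strengthens the pull as the actor faces away from the target, with a small minimum pull beyond MaxRange.
; Hits only print a debug string.
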(event `self.ReceiveBeginPlay`
  (bind _returnvalue (`GameplayStatics.GetActorOfClass` "/Game/Task_06/BP_Task_06_Target.BP_Task_06_Target_C"))
  (set `self.TargetRef` _returnvalue))

(event `self.ReceiveHit`
  (params (MyComp :type "PrimitiveComponent Object Reference") (Other :type "Actor Object Reference") (OtherComp :type "PrimitiveComponent Object Reference") (bSelfMoved :type Boolean) (HitLocation :type "Vector Structure") (HitNormal :type "Vector Structure") (NormalImpulse :type "Vector Structure") (Hit :type "HitResult Structure (by ref)"))
  (`KismetSystemLibrary.PrintString` "Hello"))

(event `self.ReceiveTick`
  (params (DeltaSeconds :type "Float (single-precision)"))
  (set `self.TargetLocation` (`self.K2_GetActorLocation` (`self.TargetRef`)))
  (set `self.TurnCoef` (`KismetMathLibrary.Dot_VectorVector` (`KismetMathLibrary.GetForwardVector` (`KismetMathLibrary.FindLookAtRotation` (`self.TargetLocation`) (`self.K2_GetActorLocation`))) (`self.GetActorForwardVector`)))
  (set `self.CurrentRange` (`KismetMathLibrary.VSize` (- (`self.K2_GetActorLocation` (`self.TargetRef`)) (`self.K2_GetActorLocation`))))
  (set `MovementComponent.Velocity` (+ (* (`self.GetActorForwardVector`) 1000.0) (* (`KismetMathLibrary.GetForwardVector` (`KismetMathLibrary.FindLookAtRotation` (`self.K2_GetActorLocation`) (`self.TargetLocation`))) (`KismetMathLibrary.MapRangeClamped` (`self.TurnCoef`) 0.0 1.0 (select `bool` (> (`self.CurrentRange`) (`self.MaxRange`)) :`false` 0.0 :`true` 5.0) 100.0))) (`self.ProjectileMovement`)))

(fn `UserConstructionScript`)