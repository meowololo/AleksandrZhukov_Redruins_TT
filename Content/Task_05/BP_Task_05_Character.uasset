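; Player character for Task 05 that rides a BP_Trajectory spline with move input disabled and throws physics balls along an aiming arrow.
; A timeline drives position along the spline, with keys and mouse wheel adjusting its play rate.
; Holding left mouse gates Tick to charge throw power and move a hit marker via projectile path prediction.
; Release launches the ball by impulse and passes the predicted flight time to the marker's destroy call.
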(event `self.ReceiveBeginPlay`
  (`Controller.SetIgnoreMoveInput` (`GameplayStatics.GetPlayerController` 0) true)
  (`self.K2_SetActorLocation` (+ (`SplineComponent.GetLocationAtDistanceAlongSpline` (`/Game/Task_05/BP_Trajectory.Spline` (`self.BP_TrajectoryRef`)) 0.0 "World") (`KismetMathLibrary.MakeVector` 0.0 0.0 (`CapsuleComponent.CapsuleHalfHeight` (`self.CapsuleComponent`)))))
  (`TimelineComponent.SetPlayRate` (`self.SplineTimeline`) 0.05)
  (bind (_direction _newtrack_0) (`Timeline|SplineTimeline`)
    (:`Update`
      (`self.K2_SetActorLocation` (+ (`SplineComponent.GetLocationAtDistanceAlongSpline` (`/Game/Task_05/BP_Trajectory.Spline` (`self.BP_TrajectoryRef`)) (`KismetMathLibrary.Lerp` 0.0 (`SplineComponent.GetSplineLength` (`/Game/Task_05/BP_Trajectory.Spline` (`self.BP_TrajectoryRef`))) _newtrack_0) "World") (`KismetMathLibrary.MakeVector` 0.0 0.0 (`CapsuleComponent.CapsuleHalfHeight` (`self.CapsuleComponent`))))))))

(event `Key|Add`
  (params (Key :type "Key Structure"))
  (bind _splinetimeline (`self.SplineTimeline`))
  (:`Pressed`
    (`TimelineComponent.SetPlayRate` _splinetimeline (+ (`TimelineComponent.GetPlayRate` _splinetimeline) 0.05))))

(event `self.ReceiveTick`
  (params (DeltaSeconds :type "Float (single-precision)"))
  (bind (_returnvalue_roll _returnvalue_pitch _returnvalue_yaw) (`KismetMathLibrary.BreakRotator` (`self.K2_GetActorRotation`)))
  (`/Engine/EditorBlueprintResources/StandardMacros.Gate` true :!label _label
    (:`Exit`
      (set `self.ThrowPower` (+ (`self.ThrowPower`) (* DeltaSeconds 1000.0)))
      (bind (_predictresult _returnvalue) (`GameplayStatics.Blueprint_PredictProjectilePath_Advanced` (make `PredictProjectilePathParams` (`SceneComponent.K2_GetComponentLocation` (`self.Arrow1`)) (* (`SceneComponent.GetForwardVector` (`self.Arrow1`)) (`self.ThrowPower`)) true 15.0 10.0 true "ECC_Visibility" _ _ 10.0 0.0 "ForOneFrame")))
      (if _returnvalue
        (`self.K2_SetActorLocationAndRotation` (`self.BP_HitPlaceRef`) (`.ImpactPoint` (`GameplayStatics.BreakHitResult` (`.HitResult` (break `PredictProjectilePathResult` _predictresult)))) (`KismetMathLibrary.MakeRotator` 0.0 0.0 _returnvalue_yaw) false false)
        (set `self.DestinationTime` (`.Time` (break `PredictProjectilePathPointData` (`.LastTraceDestination` (break `PredictProjectilePathResult` _predictresult)))))))))

(event `PrepareThrow`
  (goto _label :!via `Open`))

(event `Key|Subtract`
  (params (Key :type "Key Structure"))
  (bind _splinetimeline (`self.SplineTimeline`))
  (:`Pressed`
    (`TimelineComponent.SetPlayRate` _splinetimeline (- (`TimelineComponent.GetPlayRate` _splinetimeline) 0.05))))

(event `StopPreaparingThrow`
  (goto _label :!via `Close`))

(event `Key|MouseScrollUp`
  (params (Key :type "Key Structure"))
  (bind _splinetimeline (`self.SplineTimeline`))
  (:`Pressed`
    (`TimelineComponent.SetPlayRate` _splinetimeline (+ (`TimelineComponent.GetPlayRate` _splinetimeline) 0.01))))

(event `Key|MouseScrollDown`
  (params (Key :type "Key Structure"))
  (bind _splinetimeline (`self.SplineTimeline`))
  (:`Pressed`
    (`TimelineComponent.SetPlayRate` _splinetimeline (- (`TimelineComponent.GetPlayRate` _splinetimeline) 0.01))))

(event `Key|LeftMouseButton`
  (params (Key :type "Key Structure"))
  (bind _arrow1 (`self.Arrow1`))
  (:`Pressed`
    (`self.PrepareThrow`)
    (bind _returnvalue (`|SpawnActorFromClass` "/Game/Task_05/BP_HitPlace.BP_HitPlace_C" (`KismetMathLibrary.MakeTransform` (0.0 0.0 0.0)) "Undefined" "MultiplyWithRoot" null null))
    (set `self.BP_HitPlaceRef` _returnvalue))
  (:`Released`
    (`self.StopPreaparingThrow`)
    (bind _returnvalue_2 (`|SpawnActorFromClass` "/Game/Task_05/BP_PhysicBall.BP_PhysicBall_C" (`KismetMathLibrary.MakeTransform` (`SceneComponent.K2_GetComponentLocation` _arrow1) (`SceneComponent.K2_GetComponentRotation` _arrow1)) "Undefined" "MultiplyWithRoot" null null))
    (`PrimitiveComponent.AddImpulse` (`/Game/Task_05/BP_PhysicBall.Sphere` _returnvalue_2) (* (`SceneComponent.GetForwardVector` (`self.Arrow1`)) (`self.ThrowPower`)) "None" true)
    (set `self.ThrowPower` (`self.ThrowPowerDefault`))
    (`/Game/Task_05/BP_HitPlace.DestroyHitplace` (`self.BP_HitPlaceRef`) (`self.DestinationTime`))))

(fn `UserConstructionScript`)