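; Player character with a grappling gun that shoots a projectile to grab and carry physics objects.
; Secondary action fires BP_GrabbingProjectile from the Sphere, aimed by a camera trace, and releases it on button up.
; Hit simulating components attach to a PhysicsHandle held along camera forward each Tick, with mouse wheel adjusting distance.
; A Niagara rope tracks the projectile until its return restores the Sphere and resets state.
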(event `InputAxisKey|MouseWheelAxis`
  (params (AxisValue :type "Float (single-precision)"))
  ;[1 1 1] Grabbed item range change
  (set `self.HandleLenght` (`KismetMathLibrary.FClamp` (+ (* AxisValue 10.0) (`self.HandleLenght`)) 150.0 (`self.MaxGrabRange`))))

(event `HitItem`
  (params (HittedComp :type "PrimitiveComponent Object Reference") (HitLocation :type "Vector Structure"))
  ;[1 1 1] Grab item
  (if (`SceneComponent.IsSimulatingPhysics` HittedComp "None")
    (`PhysicsHandleComponent.GrabComponentAtLocation` (`self.PhysicsHandle`) HittedComp "None" HitLocation)
    (set `self.HandleLenght` (`KismetMathLibrary.VSize` (- (`SceneComponent.K2_GetComponentLocation` (`self.Camera`)) HitLocation)))
    (set `self.Grabbed` true)))

(event `self.ReceiveTick`
  (params (DeltaSeconds :type "Float (single-precision)"))
  (bind _camera (`self.Camera`))
  ;[1 1 1] Change GrabbedItem position
  (`|ExecutionSequence`
    (:`then_0`
      (if (`self.Grabbed`)
        (`PhysicsHandleComponent.SetTargetLocationAndRotation` :`self` (`self.PhysicsHandle`) :`NewLocation` (+ (`SceneComponent.K2_GetComponentLocation` _camera) (* (`SceneComponent.GetForwardVector` _camera) (`self.HandleLenght`))))))
    (:`then_1`
      (bind _spawnedprojectile (`self.SpawnedProjectile`)
        (:`then`
          (`NiagaraComponent.SetVariableVec3` (`self.NS_DynamicRope`) "BeamEnd" (`self.K2_GetActorLocation` _spawnedprojectile)))
        (:`else`)))))

(event `EnhancedInput|/Game/Basic/Input/IA_SecondaryAction`
  (params (ActionValue :type Boolean) (ElapsedSeconds :type "Float (double-precision)") (TriggeredSeconds :type "Float (double-precision)") (InputAction :type "InputAction Object Reference" :default "/Game/Basic/Input/IA_SecondaryAction.IA_SecondaryAction"))
  ;[1 1 1] RMB Input
  (:`Started`
    (if (not (`self.HandlerOut`))
      (`self.Shoot`)))
  (:`Completed`
    (if (`self.HandlerOut`)
      (`self.ReleaseGrabbedItem`))))

(event `Shoot`
  (bind _camera (`self.Camera`))
  (bind _ns_dynamicrope (`self.NS_DynamicRope`))
  (bind _returnvalue (`SceneComponent.K2_GetComponentLocation` _camera))
  ;[1 1 1] Shoot grabbing projectile
  (bind _outhit (`KismetSystemLibrary.LineTraceSingle` :`Start` _returnvalue :`End` (+ _returnvalue (* (`SceneComponent.GetForwardVector` _camera) (`self.MaxGrabRange`))) :`TraceChannel` "TraceTypeQuery1" :`DrawTime` 1.0))
  (bind (_bblockinghit _binitialoverlap _time _distance _location _impactpoint) (`GameplayStatics.BreakHitResult` _outhit))
  (bind _returnvalue_2 (`|SpawnActorFromClass` "/Game/Task_07/BP_GrabbingProjectile.BP_GrabbingProjectile_C" (`KismetMathLibrary.MakeTransform` (`SceneComponent.K2_GetComponentLocation` (`self.Sphere`)) (select `bool` _bblockinghit :`false` (`self.UnsuccessTrace`) :`true` (`self.SuccessTrace` _impactpoint))) "AlwaysSpawn" "MultiplyWithRoot" null null))
  (bind _output_get (set `self.SpawnedProjectile` _returnvalue_2))
  (set `/Game/Task_07/BP_GrabbingProjectile.CharRef` self _output_get)
  (`SceneComponent.SetVisibility` (`self.Sphere`) false false)
  (set `self.HandlerOut` true)
  (`ActorComponent.Activate` _ns_dynamicrope false)
  (`SceneComponent.SetVisibility` _ns_dynamicrope true false))

(event `ReleaseGrabbedItem`
  ;[1 1 1] Trigger release grabbed item
  (`PhysicsHandleComponent.ReleaseComponent` (`self.PhysicsHandle`))
  (`/Game/Task_07/BP_GrabbingProjectile.Releasehandler` (`self.SpawnedProjectile`)))

(event `HandlerReturned`
  (bind _ns_dynamicrope (`self.NS_DynamicRope`))
  ;[1 1 1] On projectile back
  (`SceneComponent.SetVisibility` (`self.Sphere`) true false)
  (set `self.HandlerOut` false)
  (set `self.Grabbed` false)
  (`ActorComponent.Deactivate` _ns_dynamicrope)
  (`SceneComponent.SetVisibility` _ns_dynamicrope false false))

(fn `SuccessTrace`
  (params (Target :type "Vector Structure (by ref)"))
  (returns (ShootRotation :type "Rotator Structure"))
  (return (`KismetMathLibrary.FindLookAtRotation` (`SceneComponent.K2_GetComponentLocation` (`self.Sphere`)) Target)))

(fn `UnsuccessTrace`
  (returns (ShootRotation :type "Rotator Structure"))
  (bind _camera (`self.Camera`))
  (return (`KismetMathLibrary.FindLookAtRotation` (`SceneComponent.K2_GetComponentLocation` (`self.Sphere`)) (+ (`SceneComponent.K2_GetComponentLocation` _camera) (* (`SceneComponent.GetForwardVector` _camera) (`self.MaxGrabRange`))))))

(fn `UserConstructionScript`)