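; Grabbing projectile that sticks to what it hits and later flies back to the owning character.
; On hit, if CharRef has nothing grabbed, it stops, attaches its sphere to the hit component and calls HitItem on the character.
; ReleaseHandler detaches it, disables collision and opens a Tick gate that steers it to the character's sphere, where it notifies and destroys itself.
; Exceeding MaxGrabRange triggers the character's ReleaseGrabbedItem once.
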(event `self.ReceiveHit`
  (params (MyComp :type "PrimitiveComponent Object Reference") (Other :type "Actor Object Reference") (OtherComp :type "PrimitiveComponent Object Reference") (bSelfMoved :type Boolean) (HitLocation :type "Vector Structure") (HitNormal :type "Vector Structure") (NormalImpulse :type "Vector Structure") (Hit :type "HitResult Structure (by ref)"))
  ;[1 1 1] ProjectileHitEvent
  (if (not (`/Game/Task_07/BP_Task_07_Character.Grabbed` (`self.CharRef`)))
    (`MovementComponent.StopMovementImmediately` (`self.ProjectileMovement`))
    (`SceneComponent.K2_AttachToComponent` (`self.Sphere`) OtherComp "None" "KeepWorld" "KeepWorld" "KeepWorld" true)
    (`/Game/Task_07/BP_Task_07_Character.HitItem` (`self.CharRef`) OtherComp HitLocation)))

(event `ReleaseHandler`
  ;[1 1 1] SendProjectile back logic
  (`self.K2_DetachFromActor` "KeepWorld" "KeepWorld" "KeepWorld")
  (`PrimitiveComponent.SetCollisionEnabled` (`self.Sphere`) "NoCollision")
  (goto _label :!via `Open`))

(event `self.ReceiveTick`
  (params (DeltaSeconds :type "Float (single-precision)"))
  (bind _charref (`self.CharRef`))
  ;[1 1 1] SendProjectile back logic
  (`|ExecutionSequence`
    (:`then_0`
      (`MovementComponent.SetUpdatedComponent` (`self.ProjectileMovement`) (`self.RootComponent`))
      (`/Engine/EditorBlueprintResources/StandardMacros.Gate` true :!label _label
        (:`Exit`
          (set `MovementComponent.Velocity` (* (`KismetMathLibrary.GetForwardVector` (`KismetMathLibrary.FindLookAtRotation` (`self.K2_GetActorLocation`) (`SceneComponent.K2_GetComponentLocation` (`/Game/Task_07/BP_Task_07_Character.Sphere` (`self.CharRef`))))) 2000.0) (`self.ProjectileMovement`))
          (if (< (`KismetMathLibrary.VSize` (- (`self.K2_GetActorLocation`) (`SceneComponent.K2_GetComponentLocation` (`/Game/Task_07/BP_Task_07_Character.Sphere` (`self.CharRef`))))) 30.0)
            (`/Game/Task_07/BP_Task_07_Character.HandlerReturned` (`self.CharRef`))
            (`self.K2_DestroyActor`)))))
    (:`then_1`
      (if (> (`KismetMathLibrary.Vector_Distance` (`self.K2_GetActorLocation`) (`SceneComponent.K2_GetComponentLocation` (`/Game/Task_07/BP_Task_07_Character.Sphere` _charref))) (`/Game/Task_07/BP_Task_07_Character.MaxGrabRange` _charref))
        (`/Engine/EditorBlueprintResources/StandardMacros.DoOnce` false
          (:`Completed`
            (`/Game/Task_07/BP_Task_07_Character.ReleaseGrabbedItem` (`self.CharRef`))))))))

(fn `UserConstructionScript`)